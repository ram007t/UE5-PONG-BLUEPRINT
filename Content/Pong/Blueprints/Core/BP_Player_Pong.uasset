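; Player-controlled Pong paddle that moves vertically while W or S is held.
; Raw key events set up and down flags, and Tick shifts the paddle a fixed step along Z, clamped to the play area and not scaled by delta time.
; BeginPlay adds an Enhanced Input mapping context, though movement uses key events, and binds to the Pong game state's game-over event to disable input.
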(event Custom|CustomEvent
  (Input|DisableInput (Game|GetPlayerController 0)))

(event EventBeginPlay
  (bind _returnvalue (Game|GetPlayerController 0))
  (bind _returnvalue_2 (PlayerController|LocalPlayerSubsystems|GetEnhancedInputLocalPlayerSubsystem _returnvalue))
  (Utilities|FlowControl|Sequence
    (:then_0
      (Utilities|IsValid _returnvalue_2
        (:Is%20Valid
          (Input|AddMappingContext _returnvalue_2 "/Game/Pong/Input/NewInputMappingContext.NewInputMappingContext" 0 "(bIgnoreAllPressedKeysUntilRelease=True,bForceImmediately=False,bNotifyUserSettings=False)")
          (bind _asbp_game_state_pong (Utilities|Casting|CastToBP_GameState_Pong (Game|GetGameState)))
          (EventDispatchers|BindEventtoGameIsOver _asbp_game_state_pong (delegate Custom|CustomEvent)))))))

(event EventTick
  (params (DeltaSeconds :type Float%20%28single-precision%29))
  (bind _returnvalue (Transformation|GetActorLocation))
  (bind _returnvalue_2 (Transformation|GetActorLocation))
  ;[0.15 0.15 0.15 0.5] movement of player paddle
  (Utilities|FlowControl|Sequence
    (:then_0
      (if (Variables|Default|Getis%20going%20up?)
        (Transformation|SetActorLocation (Math|Vector|MakeVector (.x _returnvalue) (.y _returnvalue) (Math|Float|Clamp(Float) (+ (.z _returnvalue) 2e+01) -4.5e+02 4.5e+02)) false false)))
    (:then_1
      (if (Variables|Default|Getis%20going%20down?)
        (Transformation|SetActorLocation (Math|Vector|MakeVector (.x _returnvalue_2) (.y _returnvalue_2) (Math|Float|Clamp(Float) (- (.z _returnvalue_2) 2e+01) -4.5e+02 4.5e+02)) false false)))))

(event Input|KeyboardEvents|W
  (params (Key :type Key%20Structure :default "None"))
  ;[0.15 0.15 0.15 0.5] movement of player paddle
  (:Pressed
    (Variables|Default|Setis%20going%20down? false)
    (Variables|Default|Setis%20going%20up? true))
  (:Released
    (Variables|Default|Setis%20going%20up? false)))

(event Input|KeyboardEvents|S
  (params (Key :type Key%20Structure :default "None"))
  ;[0.15 0.15 0.15 0.5] movement of player paddle
  (:Pressed
    (Variables|Default|Setis%20going%20down? true)
    (Variables|Default|Setis%20going%20up? false))
  (:Released
    (Variables|Default|Setis%20going%20down? false)))

(fn ConstructionScript)