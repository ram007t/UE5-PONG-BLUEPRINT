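; Pong game state that tracks player and AI scores and decides when the match ends.
; On BeginPlay it creates the scores widget, and each increment function updates that display, then checks both scores against the winning score.
; A win or loss sets GameOver, fires the game-over call, shows the mouse cursor and opens a match status menu with the result.
; Reset zeroes both scores and clears the widget.
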(event EventBeginPlay
  (bind _returnvalue (UserInterface|CreateWidget "/Game/Pong/Blueprints/Widgets/WBP_Scores.WBP_Scores_C"))
  (bind _output_get (Variables|Default|SetWBP_Scores_Reference _returnvalue))
  (UserInterface|Viewport|AddtoViewport _output_get 0))

(fn ConstructionScript)

(fn IncrementPlayerScore
  (bind _result (Math|Integer|IncrementInt (Variables|Default|GetPlayerScore))
    (:%20%20
      (Default|SetPlayerScore (Variables|Default|GetWBP_Scores_Reference) (Utilities|Text|ToText(Integer) _result))
      (CallFunction|CheckMatchStatus))))

(fn IncrementAIScore
  (bind _result (Math|Integer|IncrementInt (Variables|Default|GetAIScore))
    (:%20%20
      (Default|SetAIScore (Variables|Default|GetWBP_Scores_Reference) (Utilities|Text|ToText(Integer) _result))
      (CallFunction|CheckMatchStatus))))

(fn CheckMatchStatus
  (if (>= (Variables|Default|GetPlayerScore) (Variables|Default|GetWinning%20Score))
    (Variables|Default|SetGameOver? true)
    (Default|CallGameIsOver)
    (Variables|/Script/Engine.PlayerController|SetbShowMouseCursor (Game|GetPlayerController 0) true)
    (bind _returnvalue (UserInterface|CreateWidget "/Game/Pong/Blueprints/Widgets/WBP_MatchStatus_Menu.WBP_MatchStatus_Menu_C"))
    (Default|SetMatchResultText _returnvalue "YOU WON")
    (UserInterface|Viewport|AddtoViewport _returnvalue 0)
    (elif (>= (Variables|Default|GetAIScore) (Variables|Default|GetWinning%20Score))
      (Variables|Default|SetGameOver? true)
      (Default|CallGameIsOver)
      (Variables|/Script/Engine.PlayerController|SetbShowMouseCursor (Game|GetPlayerController 0) true)
      (bind _returnvalue_2 (UserInterface|CreateWidget "/Game/Pong/Blueprints/Widgets/WBP_MatchStatus_Menu.WBP_MatchStatus_Menu_C"))
      (Default|SetMatchResultText _returnvalue_2 "YOU LOSE")
      (UserInterface|Viewport|AddtoViewport _returnvalue_2 0))))

(fn Reset
  (Variables|Default|SetPlayerScore 0)
  (Variables|Default|SetAIScore 0)
  (Default|ResetScores (Variables|Default|GetWBP_Scores_Reference)))