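; Pong ball actor that launches diagonally upward to a random side and registers itself with GI_Pong on BeginPlay.
; Tick moves it by Velocity in the Y-Z plane with a swept, frame-rate-independent SetActorLocation.
; Sphere hits branch on the other actor's first tag: walls flip Z at a random speed, paddles randomise outgoing Y, always sending it upward at base Speed.
; Debug print, Z-inversion and paddle-offset bounce nodes are left unconnected.
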(event OnComponentHit(sphere_collision)
  (params (HitComponent :type Primitive%20Component%20Object%20Reference) (OtherActor :type Actor%20Object%20Reference) (OtherComp :type Primitive%20Component%20Object%20Reference) (NormalImpulse :type Vector :default "0, 0, 0") (Hit :type Hit%20Result%20Structure%20%28by%20ref%29))
  (switch name (Utilities|Array|Get(acopy) (Variables|/Script/Engine.Actor|GetTags OtherActor))
    (:TopWall
      ;[0.15 0.15 0.15 0.5] added delta seconds multiplication to - Multiply by DeltaTime to keep movement speed consistent across all frame rates
      (Variables|Default|SetVelocity (* (Math|Vector|Normalize (Math|Vector|MakeVector 0.0 (Variables|Default|GetY) -1.0)) (Math|Random|RandomFloatinRange 1.1e+03 1.4e+03))))
    (:BottomWall
      ;[0.15 0.15 0.15 0.5] added delta seconds multiplication to - Multiply by DeltaTime to keep movement speed consistent across all frame rates
      (Variables|Default|SetVelocity (* (Math|Vector|Normalize (Math|Vector|MakeVector 0.0 (Variables|Default|GetY) 1.0)) (Math|Random|RandomFloatinRange 1.1e+03 1.4e+03))))
    (:LeftPaddle
      ;[0.15 0.15 0.15 0.5] left paddle
      (Variables|Default|SetY (Math|Random|RandomFloatinRange 0.5 1.0))
      (Variables|Default|SetVelocity (* (Math|Vector|Normalize (Math|Vector|MakeVector 0.0 (Variables|Default|GetY) 1.0)) (Variables|Default|GetSpeed))))
    (:RightPaddle
      (Variables|Default|SetY (Math|Random|RandomFloatinRange -0.5 -1.0))
      (Variables|Default|SetVelocity (* (Math|Vector|Normalize (Math|Vector|MakeVector 0.0 (Variables|Default|GetY) 1.0)) (Variables|Default|GetSpeed))))))

(event EventBeginPlay
  (Utilities|FlowControl|Sequence
    (:then_0
      (Variables|Default|SetY (select (Math|Random|RandomBool) -1.0 1.0))
      (Variables|Default|SetVelocity (* (Math|Vector|Normalize (Math|Vector|MakeVector 0.0 (Variables|Default|GetY) 1.0)) (Variables|Default|GetSpeed)))
      (bind _asbp_player_pong (Utilities|Casting|CastToBP_Player_Pong (Game|Player|GetPlayerPawn 0)))
      (Variables|Default|SetAs%20BP%20Player%20Pong _asbp_player_pong))
    (:then_1
      (bind _asgi_pong (Utilities|Casting|CastToGI_Pong (Game|GetGameInstance)))
      (Default|UpdateBallReferenceinGI _asgi_pong self))))

(event EventTick
  (params (DeltaSeconds :type Float%20%28single-precision%29))
  (Variables|Default|SetNewLocation (+ (Transformation|GetActorLocation) (* (Variables|Default|GetVelocity) DeltaSeconds)))
  ;[0.15 0.15 0.15 0.5] put root component as collision, otherwise  its skipping the collisions
  (Transformation|SetActorLocation (Variables|Default|GetNewLocation) true false))

(fn ConstructionScript)