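; AI-controlled Pong paddle that tracks the ball's height while it is on the positive-Y side.
; A looping timer sets a randomly offset target Z, which Tick follows with FInterpTo to avoid jitter.
; On a ball hit, tracking pauses and a timeline eases the paddle near center until the ball crosses to negative Y, re-rolling interp speed.
; The ball reference comes from GI_Pong and refreshes through a bound event.
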(event OnComponentHit(StaticMesh)
  (params (HitComponent :type Primitive%20Component%20Object%20Reference) (OtherActor :type Actor%20Object%20Reference) (OtherComp :type Primitive%20Component%20Object%20Reference) (NormalImpulse :type Vector :default "0, 0, 0") (Hit :type Hit%20Result%20Structure%20%28by%20ref%29))
  (bind _returnvalue (Transformation|GetActorLocation))
  (if (Actor|ActorHasTag OtherActor "Ball")
    (Variables|Default|SetstopMovement? true)
    (Variables|Default|SetTargetZ_When_Paused (Math|Random|RandomFloatinRange -1e+01 1e+01))
    (bind _newtrack_0 (Timeline|Timeline PlayFromStart)
      (:Update
        (Transformation|SetActorLocation (Math|Vector|MakeVector (.x _returnvalue) (.y _returnvalue) (Math|Float|Lerp (.z _returnvalue) (Variables|Default|GetTargetZ_When_Paused) _newtrack_0)) false false)))))

(event Custom|CustomEvent
  (bind _ball_reference_local (Variables|Default|GetBall%20Reference%20Local))
  (Variables|Default|SetRandomOffSet (Math|Random|RandomFloatinRange -3e+01 3e+01))
  (Utilities|IsValid _ball_reference_local
    (:Is%20Valid
      (Variables|Default|SetTargetZ (+ (.Z (Math|Vector|BreakVector (Transformation|GetActorLocation _ball_reference_local))) (Variables|Default|GetRandomOffSet))))))

(event Custom|CustomEvent_0
  (Variables|Default|SetBall%20Reference%20Local (Variables|/Game/Pong/Blueprints/Core/GI_Pong.GI_Pong_C|GetBall_Reference (Variables|Default|GetAs%20GI%20Pong))))

(event EventBeginPlay
  (Utilities|FlowControl|Delay 1.0)
  (bind _asgi_pong (Utilities|Casting|CastToGI_Pong (Game|GetGameInstance)))
  (Variables|Default|SetAs%20GI%20Pong _asgi_pong)
  (Variables|Default|SetBall%20Reference%20Local (Variables|/Game/Pong/Blueprints/Core/GI_Pong.GI_Pong_C|GetBall_Reference (Variables|Default|GetAs%20GI%20Pong)))
  (Utilities|FlowControl|Sequence
    (:then_0
      ;[0.15 0.15 0.15 0.5] this timer updates the core values every 0.3 seconds to give human like ai feel
      (Utilities|Time|SetTimerbyEvent (delegate Custom|CustomEvent) 0.1 true))
    (:then_1
      (EventDispatchers|BindEventtoUpdateBallRef (Variables|Default|GetAs%20GI%20Pong) (delegate Custom|CustomEvent_0)))))

(event EventTick
  (params (DeltaSeconds :type Float%20%28single-precision%29))
  (bind _returnvalue (Transformation|GetActorLocation))
  (bind _ball_reference_local (Variables|Default|GetBall%20Reference%20Local))
  (bind _returnvalue_2 (Transformation|GetActorLocation _ball_reference_local))
  (bind _y (Math|Vector|BreakVector _returnvalue_2))
  (Utilities|IsValid _ball_reference_local
    (:Is%20Valid
      (if (Variables|Default|GetstopMovement?)
        (if (< _y 0.0)
          (Variables|Default|SetstopMovement? false)
          ;[0.15 0.15 0.15 0.5] this interp speed is set only when paddle actually starts moving and so its random - and not setting every tick which was causing jitter before
          (Variables|Default|SetInterpSpeed (Math|Random|RandomFloatinRange 5.0 1e+01)))
        (elif (> _y 0.0)
          (Transformation|SetActorLocation (Math|Vector|MakeVector (.x _returnvalue) (.y _returnvalue) (Math|Interpolation|FInterpTo (.z _returnvalue) (Variables|Default|GetTargetZ) (Utilities|Time|GetWorldDeltaSeconds) (Variables|Default|GetInterpSpeed))) false false))))))

(fn ConstructionScript)