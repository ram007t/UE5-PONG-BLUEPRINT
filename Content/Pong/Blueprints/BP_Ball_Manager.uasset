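; Goal zone actor for Pong that scores a point and respawns the ball when one enters its box trigger.
; An overlapping actor tagged Ball is destroyed, and the WhichSide setting decides whether the cached Pong game state increments the AI score (Player side) or the player score (AI side).
; After a short delay, a new BP_Ball spawns at the world origin unless the game is over.
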(event OnComponentBeginOverlap(Box)
  (params (OverlappedComponent :type Primitive%20Component%20Object%20Reference) (OtherActor :type Actor%20Object%20Reference) (OtherComp :type Primitive%20Component%20Object%20Reference) (OtherBodyIndex :type Integer) (bFromSweep :type Boolean) (SweepResult :type Hit%20Result%20Structure%20%28by%20ref%29))
  (bind _as_bp_game_state_pong (Variables|Default|GetAs%20BP%20Game%20State%20Pong))
  (if (Actor|ActorHasTag OtherActor "Ball")
    (Actor|DestroyActor OtherActor)
    (Utilities|FlowControl|Sequence
      (:then_0
        (switch Utilities|FlowControl|Switch|SwitchonEnum_Side (Variables|Default|GetWhichSide?)
          (:NewEnumerator0
            (Default|IncrementAIScore _as_bp_game_state_pong))
          (:NewEnumerator1
            (Default|IncrementPlayerScore _as_bp_game_state_pong))))
      (:then_1
        (Utilities|FlowControl|Delay 1.0)
        (if (not (Variables|/Game/Pong/Blueprints/Core/BP_GameState_Pong.BP_GameState_Pong_C|GetGameOver? (Variables|Default|GetAs%20BP%20Game%20State%20Pong)))
          (Game|SpawnActorfromClass "/Game/Pong/Blueprints/Core/BP_Ball.BP_Ball_C" (Math|Transform|MakeTransform "0, 0, 0") "Undefined" "MultiplyWithRoot" 0 0))))))

(event EventBeginPlay
  (bind _asbp_game_state_pong (Utilities|Casting|CastToBP_GameState_Pong (Game|GetGameState)))
  (Variables|Default|SetAs%20BP%20Game%20State%20Pong _asbp_game_state_pong))

(fn ConstructionScript)